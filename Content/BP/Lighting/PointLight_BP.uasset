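; PointLight_BP is a point light actor that applies its variables to its PointLight component.
; The Construction Script sets intensity, temperature, attenuation radius and sRGB light color from the Intensity, Temperature, Attenuation and LightColor variables.
; The event graph holds only disabled placeholder events, so the Blueprint adds no runtime behavior.
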(fn `UserConstructionScript`
  (`LightComponent.SetIntensity` (`self.PointLight`) (`self.Intensity`))
  (`LightComponent.SetTemperature` (`self.PointLight`) (`self.Temperature`))
  (`LocalLightComponent.SetAttenuationRadius` (`self.PointLight`) (`self.Attenuation`))
  (`LightComponent.SetLightColor` (`self.PointLight`) (`self.Light Color`) true))